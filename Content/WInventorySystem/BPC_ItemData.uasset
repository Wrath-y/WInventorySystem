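; BPC_ItemData is an item component that makes its owning actor a pickup in the inventory system.
; On Interact, it passes its item ID and quantity to the interactor's inventory component, if valid.
; It then looks up the DT_ItemData row and, if found, plays the pickup sound and destroys the owner, without checking the Pickup result.
; FocusTarget is a stub returning an empty value.
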(event `/Game/WInventorySystem/BPI_Interact.Interact`
  (params (Interactor :type "/Game/ThirdPerson/Blueprints/BP_ThirdPersonCharacter Object Reference"))
  (bind _bpc_inventory (`/Game/ThirdPerson/Blueprints/BP_ThirdPersonCharacter.BPC_Inventory` Interactor)
    (:`then`
      (`/Game/WInventorySystem/BPC_Inventory.Pickup` _bpc_inventory (`.RowName` (break `DataTableRowHandle` (`self.ItemID`))) (`self.ItemQuantity`))
      (bind _returnvalue (`|GetDataTableRow` "/Game/WInventorySystem/ItemData/DT_ItemData.DT_ItemData" (`.RowName` (break `DataTableRowHandle` (`self.ItemID`))))
        (:`then`
          (`GameplayStatics.PlaySoundAtLocation` (`.PIckup_2_FB730356404C0A44006B389C54B26CB9` (break `/Game/WInventorySystem/ItemData/S_ItemSFX` (`.SFX_27_3F1F60D340AF43CCE8C9029399F69799` (break `/Game/WInventorySystem/ItemData/S_ItemData` _returnvalue)))) (`Actor.K2_GetActorLocation` (`self.GetOwner`)) (struct) 1.0 1.0 0.0 null null null null)
          (`Actor.K2_DestroyActor` (`self.GetOwner`)))))
    (:`else`)))

(fn `FocusTarget`
  (returns (Message :type Text))
  (return ""))